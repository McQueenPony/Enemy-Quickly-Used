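; Base enemy Blueprint that loads its stats from a data table and exposes health functions.
; On BeginPlay, Init looks up the DT_Enemy row by Name and fills the EnemyBase struct, alongside regional bonus, begin state and begin target values; a missing row is ignored.
; Health queries and healing forward to the ACDamageSystem component.
; TakeDamage is a stub that always returns false.
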(event EventBeginPlay
  (CallFunction|Init (Variables|BeginningState|GetName)))

(event Collision|EventActorBeginOverlap
  (params (OtherActor :type Actor%20Object%20Reference)))

(event EventTick
  (params (DeltaSeconds :type Float%20%28single-precision%29)))

(fn ConstructionScript)

(fn Init
  (params (RowName :type Name))
  (bind _returnvalue (Utilities|GetDataTableRow "/Game/Enemy/DT_Enemy.DT_Enemy" RowName)
    (:then
      (Variables|BeginningState|SetEnemy%20Base (Utilities|Struct|MakeS_EnemyBase (.basehealth _returnvalue) (.resistance _returnvalue) (.canreborn? _returnvalue) (.ishuman? _returnvalue) (.abilities _returnvalue) (.weapon _returnvalue) (.givengoods _returnvalue) (Variables|BeginningState|GetRegional%20Bonus%20Value) (Variables|BeginningState|GetBegin%20State) (Variables|BeginningState|GetBegin%20Target))))
    (:RowNotFound
      _))
  (return))

(fn GetCurrentHealth
  (return (Variables|/Game/Enemy/DamageSystem/AC_DamageSystem.AC_DamageSystem_C|GetHealth (Variables|Default|GetAC_DamageSystem))))

(fn GetMaxHealth
  (return (Variables|/Game/Enemy/DamageSystem/AC_DamageSystem.AC_DamageSystem_C|GetMax%20Health (Variables|Default|GetAC_DamageSystem))))

(fn Heal
  (params (Heal%20Amount :type Float%20%28double-precision%29))
  (bind _new_health (Default|Heal (Variables|Default|GetAC_DamageSystem) Heal%20Amount))
  (return _new_health))

(fn TakeDamage
  (params (Damage%20Info :type S%20Damage%20Infomation%20Structure))
  (return false))