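; Damage system actor component in the enemy folder that tracks health, healing, blocking, invincibility and death.
; TakeDamage gates hits through CanBeDamaged, then subtracts physical and elemental damage, each reduced by resistance.
; It also accumulates per-element amounts, applying a buff and resetting the amount when the threshold check passes.
; Block, death and interrupting damage responses are reported through event calls, while DecreaseElementAmount is an empty stub.
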(fn Heal
  (params (Amount :type Float%20%28double-precision%29))
  (if (not (Variables|Default|GetIs%20Dead))
    (bind _output_get (Variables|Default|SetHealth (Math|Float|Clamp(Float) (+ Amount (Variables|Default|GetHealth)) 0.0 (Variables|Default|GetMax%20Health))))
    (return _output_get)))

(fn TakeDamage
  (params (Damage%20Info :type S%20Damage%20Infomation%20Structure))
  (bind (_damageamount _damagetype _damageresponse _shoulddamageinvincible _canbeblocked _canbeparried _shouldforceinterrupt _element _canaddbuff_ _elementamount _elementdamageamount) (Utilities|Struct|BreakS_DamageInfomation Damage%20Info))
  (bind _returnvalue (CallFunction|GetOwner))
  (LocalVariables|SetCur%20Element _element)
  (Utilities|CanbeDamaged _shoulddamageinvincible _canbeblocked
    (:Block%20Damage
      (Default|CallOnBlocked _canbeparried)
      (return false))
    (:Do%20Damage
      (if (CallFunction|GetBuffLastTime (LocalVariables|GetCur%20Element) (CallFunction|GetOwner))
        (Utilities|Map|Add (Variables|Default|GetCur%20Element%20Amount) (LocalVariables|GetCur%20Element) (+ (CallFunction|ElementAmountCalculate (LocalVariables|GetCur%20Element) _elementamount (CallFunction|GetCurElementResisatnce (LocalVariables|GetCur%20Element))) (CallFunction|GetCurElementResisatnce (LocalVariables|GetCur%20Element)))))
      (if (>= (+ (CallFunction|ElementAmountCalculate (LocalVariables|GetCur%20Element) _elementamount (CallFunction|GetCurElementResisatnce (LocalVariables|GetCur%20Element))) (CallFunction|GetCurElementResisatnce (LocalVariables|GetCur%20Element))) 0.0)
        (CallFunction|AddBuff (LocalVariables|GetCur%20Element) _returnvalue _returnvalue)
        (Utilities|Map|Add (Variables|Default|GetCur%20Element%20Amount) (LocalVariables|GetCur%20Element) 0.0))
      (bind _output_get (Variables|Default|SetHealth (- (Variables|Default|GetHealth) (+ (CallFunction|DamageReductionCalculate _damageamount (Variables|Default|GetPhysics%20Resistance) true) (CallFunction|DamageReductionCalculate _elementdamageamount (CallFunction|GetCurElementResisatnce (LocalVariables|GetCur%20Element)) false)))))
      (if (<= _output_get 0.0)
        (Variables|Default|SetIs%20Dead true)
        (Default|CallOnDeath)
        (elif (or _shouldforceinterrupt (Variables|Default|GetIs%20Interruptible))
          (Default|CallOnDamageResponse _damageresponse)))
      (return true))
    (:No%20Damage
      (return false))))

(fn DamageReductionCalculate
  (params (Damage%20Amount :type Float%20%28double-precision%29) (Resistance :type Float%20%28double-precision%29) (Is%20Physics%20Damage? :type Boolean))
  (return (/ Damage%20Amount (+ (Math|Float|SelectFloat (Variables|Default|GetPhysics%20Damage%20Constant) (Variables|Default|GetElemental%20Damage%20Constant) Is%20Physics%20Damage?) Resistance))))

(fn ElementAmountCalculate
  (params (Element :type E_ElementType%20Enum%20%28by%20ref%29 :default "NewEnumerator0") (Element%20Amount :type Float%20%28double-precision%29) (Element%20Resistance :type Float%20%28double-precision%29))
  (return (Math|Float|Clamp(Float) (+ (.Value (Utilities|Map|Find (Variables|Default|GetCur%20Element%20Amount) Element)) (* Element%20Amount (- 1.0 (/ Element%20Resistance (Variables|Default|GetElement%20Constant))))))))

(fn DecreaseElementAmount)

(fn GetCurElementResisatnce
  (params (Element :type E_ElementType%20Enum%20%28by%20ref%29 :default "NewEnumerator0"))
  (return (.Value (Utilities|Map|Find (Variables|Default|GetElement%20Resistance) Element))))

(fn Init
  (params (Physics%20Resistance :type Float%20%28double-precision%29) (Element%20Resistance :type Map%20of%20E_ElementType%20Enums%20to%20Reals :default "NewEnumerator0"))
  (Variables|Default|SetOwner (Components|GetOwner))
  (Variables|Default|SetPhysics%20Resistance Physics%20Resistance)
  (Variables|Default|SetElement%20Resistance Element%20Resistance)
  (return))

(fn GetOwner
  (return (Components|GetOwner)))