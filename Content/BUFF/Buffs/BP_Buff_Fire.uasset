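; BP_Buff_Fire is a fire-named buff whose lifecycle handlers only print debug text; it applies no gameplay effect.
; It overrides create, remove, stack-change and tick callbacks, each printing a Chinese label followed by its Message variable.
; Removal also prints the Remover's display name when valid, stack changes print the changed amount, and tick prints on every call.
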(fn BuffonCreat
  (Development|PrintString 0 (Utilities|String|Append "创建时" "_" (Variables|Default|GetMessage))))

(fn BuffonRemove
  (params (Remover :type Actor%20Object%20Reference))
  (Utilities|IsValid Remover
    (:Is%20Valid
      (Development|PrintString 0 (Utilities|String|Append "当移出时_" (Utilities|GetDisplayName Remover) "_" (Variables|Default|GetMessage))))
    (:Is%20Not%20Valid
      (Development|PrintString 0 (Utilities|String|Append "当移出时_" (Variables|Default|GetMessage))))))

(fn BuffonStackChanging
  (params (Change%20Stack :type Integer))
  (Development|PrintString 0 (Utilities|String|Append "层数变化时_" (Utilities|String|ToString(Integer) Change%20Stack) "_" (Variables|Default|GetMessage))))

(fn BuffonTick
  (params (Delta%20Time :type Float%20%28double-precision%29))
  (Development|PrintString 0 (Utilities|String|Append "Tick时_" (Variables|Default|GetMessage))))