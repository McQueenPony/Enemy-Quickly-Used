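; Actor component that manages buffs, creating them by ID from DT_BuffConfig and tracking their stacking, ticking and removal.
; AddBuff queues new buff objects; each tick merges that queue, ticks current buffs, then removes those whose tick returns true.
; A repeated ID stacks onto the existing buff until max, then extends or resets duration per its config rule.
; Buff objects receive create, stack-change and remove callbacks.
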(event EventBeginPlay)

(event EventTick
  (params (DeltaSeconds :type Float%20%28single-precision%29))
  (CallFunction|BuffsTick DeltaSeconds))

(fn AddBuff
  (params (ID :type Name) (Creator :type Actor%20Object%20Reference) (Target :type Actor%20Object%20Reference))
  (bind _returnvalue (Utilities|GetDataTableRow "/Game/BUFF/DT_BuffConfig.DT_BuffConfig" ID)
    (:then
      (bind _returnvalue_2 (Game|ConstructObjectfromClass (Utilities|Struct|BreakF_BuffConfig _returnvalue)))
      (Default|Init _returnvalue_2 _returnvalue Creator Target 1)
      (Utilities|Array|Add (Variables|Default|GetWaiting%20Add%20Buffs) _returnvalue_2))))

(fn RemoveBuff
  (params (Delete%20Buff :type BP%20Buff%20Base%20Object%20Reference) (Remover :type Actor%20Object%20Reference))
  (bind _returnvalue (Utilities|Array|RemoveItem (Variables|Default|GetCur%20Buffs) Delete%20Buff))
  (if _returnvalue
    (Default|BuffonRemove Delete%20Buff Remover)))

(fn FindBuffsbyIDReturnIndex
  (params (ID :type Name) (Buffs :type Array%20of%20BP%20Buff%20Base%20Object%20References))
  (for (_array_element _array_index) Buffs
    (if (== (Utilities|Struct|BreakF_BuffConfig (Variables|/Game/BUFF/BP_Buff_Base.BP_Buff_Base_C|GetBuff%20Config _array_element)) ID)
      (return true _array_index _array_element)))
  (return false 0 0))

(fn BuffsTick
  (params (Delta%20Time :type Float%20%28double-precision%29))
  (Utilities|FlowControl|Sequence
    (:then_0
      (|HandleWaitAddBuffs))
    (:then_1
      (|HandleCurrantBuffs))
    (:then_2
      (|HandleWaitRemoveBuffs))))