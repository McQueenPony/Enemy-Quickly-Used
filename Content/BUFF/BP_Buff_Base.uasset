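; Base buff class that tracks one buff's config, creator, target, stack count and timers, with empty create, remove, stack-change and period hooks.
; BuffOnTick counts down duration unless the buff is permanent, and fires periodic effects when their timer nears zero.
; On timeout, the configured stack rule either clears the buff or drops a stack and restarts duration.
; The tick returns true when the buff has expired.
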(fn BuffonTick
  (params (Delta%20Time :type Float%20%28double-precision%29))
  (|TimeSettings)
  (if (and (<= (Variables|RunTimeVar|GetCurDuration) 0.0) (not (Utilities|Struct|BreakF_BuffConfig (Variables|Default|GetBuff%20Config))))
    (switch Utilities|FlowControl|Switch|SwitchonE_TimeOutStackRule (Utilities|Struct|BreakF_BuffConfig (Variables|Default|GetBuff%20Config))
      (:NewEnumerator0
        _)
      (:NewEnumerator1
        (bind _result (Math|Integer|DecrementInt (Variables|RunTimeVar|GetCurStack))
          (:%20%20
            (CallFunction|BuffonStackChanging -1)
            (if (<= _result 0)
              _
              (else
                (Variables|RunTimeVar|SetCurDuration (Utilities|Struct|BreakF_BuffConfig (Variables|Default|GetBuff%20Config)))
                (return false)))))))
    (if (and (<= (Variables|RunTimeVar|GetCurPeroid) 0.05) (Utilities|Struct|BreakF_BuffConfig (Variables|Default|GetBuff%20Config)))
      (CallFunction|BuffonPeriod))
    (return true)
    (elif (and (<= (Variables|RunTimeVar|GetCurPeroid) 0.05) (Utilities|Struct|BreakF_BuffConfig (Variables|Default|GetBuff%20Config)))
      (CallFunction|BuffonPeriod)
      (Variables|RunTimeVar|SetCurPeroid (Utilities|Struct|BreakF_BuffConfig (Variables|Default|GetBuff%20Config)))
      (return false)
      (else
        (return false)))))

(fn BuffonCreat)

(fn BuffonRemove
  (params (Remover :type Actor%20Object%20Reference)))

(fn BuffonStackChanging
  (params (Change%20Stack :type Integer)))

(fn BuffonPeriod)

(fn Init
  (params (Buff%20Config :type F%20Buff%20Config%20Structure) (Creator :type Actor%20Object%20Reference) (Target :type Actor%20Object%20Reference) (CurStack :type Integer))
  (Variables|Default|SetBuff%20Config Buff%20Config)
  (Variables|RunTimeVar|SetCreator Creator)
  (Variables|RunTimeVar|SetTarget Target)
  (Variables|RunTimeVar|SetCurStack CurStack)
  (Variables|RunTimeVar|SetCurDuration (.Duration (Utilities|Struct|BreakF_BuffConfig (Variables|Default|GetBuff%20Config))))
  (Variables|RunTimeVar|SetCurPeroid (.Peroid (Utilities|Struct|BreakF_BuffConfig (Variables|Default|GetBuff%20Config)))))

(fn GetBuffID
  (return (Utilities|Struct|BreakF_BuffConfig (Variables|Default|GetBuff%20Config))))

(fn IsMaxStack
  (return (>= (Variables|RunTimeVar|GetCurStack) (Utilities|Struct|BreakF_BuffConfig (Variables|Default|GetBuff%20Config)))))

(fn AddTime(Duration)
  (Variables|RunTimeVar|SetCurDuration (+ (Variables|RunTimeVar|GetCurDuration) (Utilities|Struct|BreakF_BuffConfig (Variables|Default|GetBuff%20Config)))))

(fn ResetTime(Duration)
  (Variables|RunTimeVar|SetCurDuration (Utilities|Struct|BreakF_BuffConfig (Variables|Default|GetBuff%20Config))))